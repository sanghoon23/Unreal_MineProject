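; Pickup display actor that shows an animated item mesh with a platform, hologram glow and colored lights.
; The construction script applies the configurable item mesh, the materials for item, platform and glow, and one shared color across all the lights.
; On BeginPlay, a boolean selects hovering or spinning, each a self-restarting MoveComponentTo loop that bobs or yaws the item.
; The graphs contain only this visual setup, with no collection logic.
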(event Custom|Spining_Animate
  (bind _pickupitem (Variables|Default|GetPickUpItem))
  (bind _pickupitem_2 (Variables|Default|GetPickUpItem))
  (bind _relativerotation (Variables|/Script/Engine.SceneComponent|GetRelativeRotation _pickupitem_2))
  (bind (_roll _pitch _yaw) (Math|Rotator|BreakRotator _relativerotation))
  ;[1 1 1] Spining Animation: (This move the Item around the speed can be control using the "Over Time" Float).
  (Components|MoveComponentTo _pickupitem (Variables|/Script/Engine.SceneComponent|GetRelativeLocation _pickupitem) (Math|Rotator|MakeRotator _roll _pitch (+ _yaw 1.8e+02)) false false 2.0 false)
  (CallFunction|SpiningAnimate))

(event Custom|Hovering_Animate
  (bind _pickupitem (Variables|Default|GetPickUpItem))
  (bind _pickupitem_2 (Variables|Default|GetPickUpItem))
  ;[1 1 1] Hovering Animation: (This move the Item up and down).
  (Components|MoveComponentTo _pickupitem (+ (Variables|/Script/Engine.SceneComponent|GetRelativeLocation _pickupitem) "0, 0,5.000000") (Variables|/Script/Engine.SceneComponent|GetRelativeRotation (Variables|Default|GetPickUpItem)) false false 1.0 false)
  (Components|MoveComponentTo _pickupitem_2 (- (Variables|/Script/Engine.SceneComponent|GetRelativeLocation _pickupitem_2) "0, 0,5.000000") (Variables|/Script/Engine.SceneComponent|GetRelativeRotation (Variables|Default|GetPickUpItem)) false false 1.0 false)
  (CallFunction|HoveringAnimate))

(event EventBeginPlay
  ;[1 1 1] Starts a animation type.
  (if (Variables|Animation|GetHoverOrSpin_Animation?)
    (CallFunction|HoveringAnimate)
    (else
      (CallFunction|SpiningAnimate))))

(fn ConstructionScript
  (Components|StaticMesh|SetStaticMesh (Variables|Default|GetPickUpItem) (Variables|VisualSettings|GetItemPickUp_MESH))
  (Rendering|Material|SetMaterial (Variables|Default|GetPickUpItem) 0 (Variables|VisualSettings|GetItemPickUp_MAT))
  (Rendering|Material|SetMaterial (Variables|Default|GetItemPickup_Platform) 0 (Variables|VisualSettings|GetItemPickUpPlatform_MAT))
  (Rendering|Material|SetMaterial (Variables|Default|GetHologramGlow) 0 (Variables|VisualSettings|GetHologramGlow_MAT))
  (Rendering|Components|Light|SetLightColor (Variables|Default|GetPointLight4) (Variables|VisualSettings|GetLightColour) true))